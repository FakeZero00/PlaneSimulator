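; Player plane Blueprint that flies by moving along its local forward axis each Tick, with text-render readouts for speed, distance, coins and time.
; Speed integrates acceleration, drag and braking up to a maximum, while roll and mouse inputs rotate the actor.
; Below 80 km/h it stalls: physics and gravity take over and a stall warning appears.
; Helper functions convert between km/h and cm/s.
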(event EventBeginPlay
  (Variables|Default|SetCurrentSpeed 0.0)
  (Variables|Default|SetCurrentPosition (Transformation|GetActorLocation))
  (Variables|Default|SetGetCoin 0)
  (Variables|Default|SetTime 0.0))

(event Collision|EventActorBeginOverlap
  (params (OtherActor :type Actor%20Object%20Reference)))

(event EventTick
  (params (DeltaSeconds :type Float%20%28single-precision%29))
  (bind _plane (Variables|Default|GetPlane))
  (bind _mouseinput (Variables|Default|GetMouseInput))
  (bind _output_get (Variables|Default|SetCurrentSpeed (Math|Float|Clamp(Float) (- (+ (Variables|Default|GetCurrentSpeed) (* (Variables|Default|GetUseAccel) (CallFunction|Km/h2cm/s (Variables|Default|GetAcceleration)) DeltaSeconds)) (+ (* (CallFunction|Km/h2cm/s (Variables|Default|GetDrag)) DeltaSeconds) (* (Variables|Default|GetUseBreak) (Variables|Default|GetBreak) DeltaSeconds))) 0.0 (CallFunction|Km/h2cm/s (Variables|Default|GetMaxSpeed)))))
  (Physics|SetSimulatePhysics _plane (not (>= _output_get (CallFunction|Km/h2cm/s 8e+01))))
  (Physics|SetEnableGravity _plane (not (>= _output_get (CallFunction|Km/h2cm/s 8e+01))))
  (Rendering|SetVisibility (Variables|Default|GetTextRender_Stall) (not (>= _output_get (CallFunction|Km/h2cm/s 8e+01))) false)
  (Rendering|Components|TextRender|SetText (Variables|Default|GetTextRender_Speed) (Utilities|Text|FormatText "Speed: {CurrentSpeed}km/s" (Utilities|Text|ToText(Float) (CallFunction|Cm/s2km/h (Variables|Default|GetCurrentSpeed)) "HalfToEven" false true 1 324 2 2)))
  (Transformation|AddActorLocalRotation (Math|Rotator|MakeRotator (* (Variables|Default|GetRollInput) (Variables|Default|GetRollSpeed)) (* (.y _mouseinput) (Variables|Default|GetPitchSpeed)) (.x _mouseinput)) false false)
  (Transformation|AddActorLocalOffset (Math|Vector|MakeVector (* (Variables|Default|GetCurrentSpeed) DeltaSeconds) 0.0 0.0) false false)
  (bind _output_get_2 (Variables|Default|SetTotalDistance (+ (Variables|Default|GetTotalDistance) (Math|Vector|VectorLength (- (Transformation|GetActorLocation) (Variables|Default|GetCurrentPosition))))))
  (Variables|Default|SetCurrentPosition (Transformation|GetActorLocation))
  (Rendering|Components|TextRender|SetText (Variables|Default|GetTextRender_Total_Distance) (Utilities|Text|FormatText "Total Distance: {TotalDistance}m" (Utilities|Text|ToText(Float) (/ _output_get_2 1e+02) "HalfToEven" false true 1 324 2 2)))
  (Rendering|Components|TextRender|SetText (Variables|Default|GetTextRender_Total_Coin) (Utilities|Text|FormatText "Total Coin: {GetCoin}/{AllCoin}" (Variables|Default|GetGetCoin) (Variables|Default|GetAllCoin)))
  (bind _output_get_3 (Variables|Default|SetTime (+ (Variables|Default|GetTime) DeltaSeconds)))
  (Rendering|Components|TextRender|SetText (Variables|Default|GetTextRender_Total_Time) (Utilities|Text|FormatText "Total Time: {Time}" (Utilities|Text|ToText(Float) _output_get_3 "HalfToEven" false true 1 324 1 1))))

(fn ConstructionScript)

(fn Km/h2cm/s
  (params (km/h :type Float%20%28double-precision%29))
  (return (/ (* km/h 1e+05) 3.6e+03)))

(fn Cm/s2km/h
  (params (cm/s :type Float%20%28double-precision%29))
  (return (* (/ cm/s 1e+05) 3.6e+03)))