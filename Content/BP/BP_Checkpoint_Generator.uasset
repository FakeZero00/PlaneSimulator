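; Spline-driven generator that lays out a checkpoint course with collectible coins for BP_Plane.
; The construction script builds the spline from ControlPoints, placing instanced checkpoints and path markers at set intervals, with random path slots becoming separate coin mesh components.
; BeginPlay gives the player plane the coin total and binds coin overlaps.
; An overlap plays a sound and, for a BP_Plane, increments its count and destroys the coin.
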(event Custom|OnComponentBeginOverlap_Event
  (params (OverlappedComponent :type Primitive%20Component%20Object%20Reference) (OtherActor :type Actor%20Object%20Reference) (OtherComp :type Primitive%20Component%20Object%20Reference) (OtherBodyIndex :type Integer) (bFromSweep :type Boolean) (SweepResult :type Hit%20Result%20Structure%20%28by%20ref%29))
  (Audio|PlaySoundatLocation "/Engine/VREditor/Sounds/VR_open.VR_open" (Transformation|GetActorLocation OtherActor) "0, 0, 0" 1.0 1.0 0.0 0 0 0 0)
  (bind _asbp_plane (Utilities|Casting|CastToBP_Plane OtherActor))
  (Variables|/Game/BP/BP_Plane.BP_Plane_C|SetGetCoin _asbp_plane (+ (Variables|/Game/BP/BP_Plane.BP_Plane_C|GetGetCoin _asbp_plane) 1))
  (Components|DestroyComponent OverlappedComponent))

(event EventBeginPlay
  (bind _coins (Variables|Default|GetCoins))
  (bind _returnvalue (Utilities|Array|Length _coins))
  (bind _asbp_plane (Utilities|Casting|CastToBP_Plane (Game|Player|GetPlayerPawn 0)))
  (Variables|/Game/BP/BP_Plane.BP_Plane_C|SetAllCoin _asbp_plane _returnvalue)
  (for _index (range 0 (- _returnvalue 1))
    (Collision|AssignOnComponentBeginOverlap (Utilities|Array|Get(acopy) (Variables|Default|GetCoins) _index) (delegate Custom|OnComponentBeginOverlap_Event))))

(event Collision|EventActorBeginOverlap
  (params (OtherActor :type Actor%20Object%20Reference)))

(event EventTick
  (params (DeltaSeconds :type Float%20%28single-precision%29)))

(fn ConstructionScript
  (bind _spline (Variables|Default|GetSpline))
  (bind _spline_2 (Variables|Default|GetSpline))
  (bind _spline_3 (Variables|Default|GetSpline))
  (Components|InstancedStaticMesh|ClearInstances (Variables|Default|GetHierarchicalInstancedStaticMesh_Checkpoint))
  (Spline|SetSplinePoints _spline (Variables|Default|GetControlPoints) "Local" true)
  (for _index (range 0 (Math|Float|Truncate (/ (Spline|GetSplineLength _spline) (Variables|Default|GetCheckPointInterval))))
    (Components|InstancedStaticMesh|AddInstance (Variables|Default|GetHierarchicalInstancedStaticMesh_Checkpoint) (Math|Transform|MakeTransform (Spline|GetLocationatDistanceAlongSpline _spline_2 (* _index (Variables|Default|GetCheckPointInterval)) "Local") (Spline|GetRotationatDistanceAlongSpline _spline_2 (* _index (Variables|Default|GetCheckPointInterval)) "Local") "1.000000,1.000000,1.000000") false))
  (for _index_2 (range 0 (Math|Float|Truncate (/ (Spline|GetSplineLength (Variables|Default|GetSpline)) (Variables|Default|GetPathInterval))))
    (if (>= (Math|Random|RandomIntegerinRange 0 10) 4)
      (Components|InstancedStaticMesh|AddInstance (Variables|Default|GetHierarchicalInstancedStaticMesh_Path) (Math|Transform|MakeTransform (Spline|GetLocationatDistanceAlongSpline _spline_3 (* _index_2 (Variables|Default|GetPathInterval)) "Local") (Spline|GetRotationatDistanceAlongSpline _spline_3 (* _index_2 (Variables|Default|GetPathInterval)) "Local") "1.000000,1.000000,1.000000") false)
      (else
        (bind _returnvalue (AddComponent|AddStaticMeshComponent false (Math|Transform|MakeTransform (Spline|GetLocationatDistanceAlongSpline _spline_3 (* _index_2 (Variables|Default|GetPathInterval)) "Local") (Spline|GetRotationatDistanceAlongSpline _spline_3 (* _index_2 (Variables|Default|GetPathInterval)) "Local") "1.000000,1.000000,1.000000")))
        (Utilities|Array|Add (Variables|Default|GetCoins) _returnvalue))))
  (Variables|Default|SetPathLengtn (Spline|GetSplineLength (Variables|Default|GetSpline))))